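; Command ship that flies to ordered destinations and automatically fires missiles at enemies in range.
; MoveShip requests an async CPathVolume path and steps through it with timeline lerps, falling back to a straight lerp if pathfinding fails.
; Looping timers drive nearest-enemy search and missile launches from mesh sockets.
; Upgrades raise capped levels for speed, range, reload (restarting the fire timer) and weapon, changing missile class and adding secondary missiles.
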(event `self.ReceiveBeginPlay`
  ;[1 1 1] initialize
  (`self.Set First CPath Vol`)
  (set `self.AttackRange ` 2000.0)
  (set `self.MissileClass  ` "/Game/BluePrints/Missile/BP_Missil_Red.BP_Missil_Red_C")
  (set `self.FireInterval` 0.3)
  ;;[1 1 1] loop to find enemy and fire missile
  (`KismetSystemLibrary.K2_SetTimerDelegate` (`|CreateDelegate` :!event `Find Nearest Enemy CS`) 0.05 true)
  (bind _returnvalue (`KismetSystemLibrary.K2_SetTimerDelegate` (`|CreateDelegate` :!event `Fire Missiles`) (`self.FireInterval`) true))
  ;;[1 1 1] Need for upgrade
  (set `self.FireMissileEvent` _returnvalue))

(event `MoveShip`
  (params (destination :type "Vector Structure"))
  (bind (_returnvalue_roll _returnvalue_pitch _returnvalue_yaw) (`KismetMathLibrary.BreakRotator` (`KismetMathLibrary.FindLookAtRotation` (`KismetMathLibrary.MakeVector` (.x (`self.StartLocation`)) (.y (`self.StartLocation`))) (`KismetMathLibrary.MakeVector` (.x (`self.TargetLocation`)) (.y (`self.TargetLocation`))))))
  ;[1 1 1] smooth move
  (set `self.StartLocation` (`self.K2_GetActorLocation`))
  (set `self.TargetLocation` (`KismetMathLibrary.MakeVector` destination_X destination_Y (+ destination_Z 50.0)))
  (if (`self.IsMoving`)
    (set `self.NewDesWhileMoving` true)
    (else
      (set `self.IsMoving` true)
      (set `self.NewDesWhileMoving` false)))
  (bind (_ascpath_volume _path) (`self.GetPath`)
    (:`Success`
      (set `self.Path` _path)
      (set `self.CurrentPathIndex ` 2)
      (`self.MoveToNextLocation`)
      (`CPathVolume.DrawDebugPath` _ascpath_volume _path 50.0 true (struct :`B` 255 :`R` 255 :`A` 255)))
    (:`FailedToFindPath`
      (`KismetSystemLibrary.PrintString` "get stucked")
      (bind _output_get (set `self.TargetRotation` (`KismetMathLibrary.MakeRotator` _returnvalue_roll _returnvalue_pitch (+ -90.0 _returnvalue_yaw 0.0))))
      (`self.K2_SetActorRotation` _output_get)
      (`TimelineComponent.SetPlayRate` (`self.MoveTimeline`) (/ (`self.ShipSpeed`) (`KismetMathLibrary.Vector_Distance` (`self.StartLocation`) (`self.TargetLocation`))))
      (bind (_direction _move) (`Timeline|Timeline` :!via `PlayFromStart`)
        (:`Update`
          (`self.K2_SetActorLocation` (`KismetMathLibrary.VLerp` (`self.StartLocation`) (`self.TargetLocation`) _move)))))))

(event `UpgradeWeapon`
  ;[1 1 1] Implement upgrade interface
  (if (not (>= (`self.AttackLevel`) 3))
    (bind _output_get (set `self.AttackLevel` (+ (`self.AttackLevel`) 1)))
    (if (>= _output_get 2)
      (set `self.MissileClass  ` "/Game/BluePrints/Missile/BP_Missile_Blue.BP_Missile_Blue_C"))))

(event `MoveToNextLocation`
  (bind _returnvalue (`KismetMathLibrary.Vector_Distance` (`self.StartLocation`) (`self.TargetLocation`)))
  (bind _output_worldlocation (break `CPathNode` (`|GetArrayItem` (`self.Path`) (`self.CurrentPathIndex `))))
  (bind (_returnvalue_roll _returnvalue_pitch _returnvalue_yaw) (`KismetMathLibrary.BreakRotator` (`KismetMathLibrary.FindLookAtRotation` (`KismetMathLibrary.MakeVector` (.x (`self.StartLocation`)) (.y (`self.StartLocation`))) (`KismetMathLibrary.MakeVector` (.x (`self.TargetLocation`)) (.y (`self.TargetLocation`))))))
  (set `self.NewDesWhileMoving` false)
  (set `self.StartLocation` (`self.K2_GetActorLocation`))
  (set `self.TargetLocation` _output_worldlocation)
  (set `self.CurrentPathIndex ` (+ (`self.CurrentPathIndex `) 1))
  (if (> _returnvalue 100.0)
    (bind _output_get (set `self.TargetRotation` (`KismetMathLibrary.MakeRotator` _returnvalue_roll _returnvalue_pitch (+ -90.0 _returnvalue_yaw 0.0))))
    (`self.K2_SetActorRotation` _output_get)
    (`TimelineComponent.SetPlayRate` (`self.MoveTimeline`) (/ (`self.ShipSpeed`) _returnvalue))
    (bind (_direction _move) (`Timeline|MoveTimeline` :!via `PlayFromStart` :!label _label)
      (:`Update`
        (if (`self.NewDesWhileMoving`)
          (goto _label :!via `Stop`)
          (else
            (`self.K2_SetActorLocation` (`KismetMathLibrary.VLerp` (`self.StartLocation`) (`self.TargetLocation`) _move)))))
      (:`Finished`
        (if (< (`self.CurrentPathIndex `) (`KismetArrayLibrary.Array_Length` (`self.Path`))) :!label _label_2
          (if (`self.NewDesWhileMoving`)
            (set `self.IsMoving` false :!label _label_3)
            (else
              (`self.MoveToNextLocation`)))
          (else
            (goto _label_3)))))
    (else
      (goto _label_2))))

(event `/Game/BluePrints/Interfaces/BI_Upgrade.Upgrade`
  (params (UpgradeClassType :type "Actor Class Reference") (UpgradeActor :type "Actor Object Reference") (WeaponAttack :type Boolean) (Reload :type Boolean) (MovementSpeed :type Boolean) (AttackRange :type Boolean))
  ;[1 1 1] Implement upgrade interface
  (if (== UpgradeClassType "BPCommandShip_C")
    (if WeaponAttack
      (`self.UpgradeWeapon`))
    (`self.UpgradeReload` Reload)
    (`self.UpgradeSpeed` MovementSpeed)
    (`self.UpgradeRange` AttackRange)))

(fn `Find Nearest Enemy CS`
  (bind (_nearestenemy _enemieswithinrange) (`/Game/BluePrints/Utilities/BP_UtilityLibrary.Find Nearest Enemy` self "/Game/BluePrints/DummyEnemy/BP_DummyEnemy.BP_DummyEnemy_C" (`self.AttackRange `)))
  (set `self.TargetEnemy` _nearestenemy)
  (set `self.AllEnemiesWithinRange` _enemieswithinrange))

(fn `Fire Missiles`
  (bind _allenemieswithinrange (`self.AllEnemiesWithinRange`))
  (`/Engine/EditorBlueprintResources/StandardMacros.IsValid` (`self.TargetEnemy`)
    (:`Is Valid`
      ;[1 1 1] Spawn main missile and set the missle target
      (bind _returnvalue (`|SpawnActorFromClass` (`self.MissileClass  `) (`KismetMathLibrary.MakeTransform` (`SceneComponent.GetSocketLocation` (`self.StaticMesh`) "MainBattery")) "Undefined" "MultiplyWithRoot" null null))
      (bind _asbp_missile_parent (cast `/Game/BluePrints/Missile/BP_Missile_Parent` _returnvalue))
      (`/Game/BluePrints/Missile/BP_Missile_Parent.SetTargetEnemy` _asbp_missile_parent (`self.TargetEnemy`))
      ;[1 1 1] Create secondary missiles
      (if (>= (`self.AttackLevel`) 3)
        (`|ExecutionSequence`
          (:`then_0`
            (bind _returnvalue_2 (`|SpawnActorFromClass` "/Game/BluePrints/Missile/BP_Missile_Secondaries.BP_Missile_Secondaries_C" (`KismetMathLibrary.MakeTransform` (`SceneComponent.GetSocketLocation` (`self.StaticMesh`) "cannon1")) "Undefined" "MultiplyWithRoot" null null))
            (`/Game/BluePrints/Missile/BP_Missile_Parent.SetTargetEnemy` _returnvalue_2 (`|GetArrayItem` _allenemieswithinrange)))
          (:`then_1`
            (bind _returnvalue_3 (`|SpawnActorFromClass` "/Game/BluePrints/Missile/BP_Missile_Secondaries.BP_Missile_Secondaries_C" (`KismetMathLibrary.MakeTransform` (`SceneComponent.GetSocketLocation` (`self.StaticMesh`) "cannon2")) "Undefined" "MultiplyWithRoot" null null))
            (`/Game/BluePrints/Missile/BP_Missile_Parent.SetTargetEnemy` _returnvalue_3 (`|GetArrayItem` _allenemieswithinrange (`KismetArrayLibrary.Array_LastIndex` _allenemieswithinrange)))))
        (else
          (return))))))

(fn `Set First CPath Vol`
  (bind _outactors (`GameplayStatics.GetAllActorsOfClass` "/Script/CPathfinding.CPathVolume"))
  (set `self.CPathVol` (`|GetArrayItem` _outactors))
  (return))

(fn `UpgradeRange`
  (params (Condition :type Boolean))
  (if Condition
    (if (< (`self.RangeLevel`) 2)
      (set `self.RangeLevel` (+ (`self.RangeLevel`) 1))
      (set `self.AttackRange ` (+ (`self.AttackRange `) 500.0)))))

(fn `UpgradeReload`
  (params (Condition :type Boolean))
  (if Condition
    (if (< (`self.ReloadLevel`) 2)
      (set `self.ReloadLevel` (+ (`self.ReloadLevel`) 1))
      (bind _output_get (set `self.FireInterval` (/ (`self.FireInterval`) 2.0)))
      (`KismetSystemLibrary.K2_ClearAndInvalidateTimerHandle` (`self.FireMissileEvent`))
      (bind _returnvalue (`KismetSystemLibrary.K2_SetTimerDelegate` (`|CreateDelegate` :!event `Fire Missiles`) _output_get true))
      (set `self.FireMissileEvent` _returnvalue))))

(fn `UpgradeSpeed`
  (params (Condition :type Boolean))
  (if Condition
    (if (< (`self.SpeedLevel`) 2)
      (set `self.SpeedLevel` (+ (`self.SpeedLevel`) 1))
      (set `self.ShipSpeed` (+ (`self.ShipSpeed`) 1000.0)))))

(fn `UserConstructionScript`)