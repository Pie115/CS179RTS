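; Blueprint function library of enemy-targeting queries, finding and ranking actors of a given class by distance.
; Searches scan all actors of the class for the nearest within range of an actor or fixed location; the actor-based search uses a shared helper and also gathers enemies in range.
; Gate-based sorting pairs each enemy with its distance in structs, calls SortEnemiesByDistance, then returns the ordered actors.
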(fn `Find Nearest Enemy`
  (params (SearchingActor :type "Actor Object Reference") (SearchedActor :type "Actor Class Reference") (SearchingRange :type "Float (double-precision)"))
  (returns (NearestEnemy :type "Actor Object Reference") (EnemiesWithinRange :type "Array of Actor Object Reference"))
  (locals (CurrentShortest :type "Float (double-precision)") (NearEnemy :type "Actor Object Reference") (Enemies :type "Array of Actor Object Reference"))
  ;[1 1 1] find the nearest searched actor (enemy) and all enemies within range around the searching actor
  (set `local.CurrentShortest` SearchingRange)
  (bind _outactors (`GameplayStatics.GetAllActorsOfClass` null SearchedActor))
  (for _array_element _outactors
    (bind _returnvalue (`Actor.GetDistanceTo` _array_element SearchingActor))
    (if (<= _returnvalue (`local.SearchingRange`))
      (`KismetArrayLibrary.Array_Add` (`local.Enemies`) _array_element)
      (if (< _returnvalue (`local.CurrentShortest`))
        (set `local.CurrentShortest` _returnvalue)
        (set `local.NearEnemy` _array_element))))
  (return (`local.NearEnemy`) (`local.Enemies`)))

(fn `Find Nearest Enemy by Static Location`
  (params (SearchingLocation :type "Vector Structure") (SearchedActor :type "Actor Class Reference") (SearchingRange :type "Float (double-precision)"))
  (returns (NearestEnemy :type "Actor Object Reference"))
  (locals (CurrentShortest :type "Float (double-precision)") (NearEnemy :type "Actor Object Reference"))
  (set `local.CurrentShortest` SearchingRange)
  (bind _outactors (`GameplayStatics.GetAllActorsOfClass` null SearchedActor))
  (for _array_element _outactors
    (bind _returnvalue (`KismetMathLibrary.Vector_Distance` SearchingLocation (`Actor.K2_GetActorLocation` _array_element)))
    (if (< _returnvalue (`local.CurrentShortest`))
      (set `local.CurrentShortest` _returnvalue)
      (set `local.NearEnemy` _array_element)))
  (return (`local.NearEnemy`)))

(fn `Get Sorted Enemies by Distance`
  (params (EnemyClass :type "Actor Class Reference") (GateLocation :type "Vector Structure"))
  (returns (SortedEnemies :type "Array of Actor Object Reference"))
  (locals (`EnemyDistanceArray ` :type "Array of EnemyDistanceStruct Structure") (`SortedEnemyArray ` :type "Array of Actor Object Reference"))
  ;[1 1 1] get all distance
  (bind _outactors (`GameplayStatics.GetAllActorsOfClass` null EnemyClass))
  (for _array_element _outactors
    (`KismetArrayLibrary.Array_Add` (`local.EnemyDistanceArray `) (make `EnemyDistanceStruct` _array_element (`KismetMathLibrary.Vector_Distance` (`Actor.K2_GetActorLocation` _array_element) GateLocation))))
  ;[1 1 1] return sorted enemies
  (bind _sortedenemies (`MyBlueprintFunctionLibrary.SortEnemiesByDistance` (`local.EnemyDistanceArray `)))
  (for _array_element_2 _sortedenemies
    (`KismetArrayLibrary.Array_Add` (`local.SortedEnemyArray `) (`.Enemy` (break `EnemyDistanceStruct` _array_element_2))))
  (return (`local.SortedEnemyArray `)))