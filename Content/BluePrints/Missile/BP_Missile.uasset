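; BP_Missile is a homing projectile that chases an assigned enemy and damages dummy enemies on impact.
; SetTargetEnemy stores the target, and Tick re-aims the ProjectileMovement velocity straight at it every frame at initial speed, with no gradual turning.
; A Sphere hit on a BP_DummyEnemy applies fixed damage and destroys the missile, while hits on other actors are ignored.
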(event `SetTargetEnemy`
  (params (Eenemy :type "Actor Object Reference"))
  ;[1 1 1] set the target enemy
  (set `self.Target` Eenemy))

(event `self.ReceiveTick`
  (params (DeltaSeconds :type "Float (single-precision)"))
  (bind _target (`self.Target`))
  (bind _projectilemovement (`self.ProjectileMovement`))
  ;[1 1 1] add velocity so the missle can chase after the enemy
  (`/Engine/EditorBlueprintResources/StandardMacros.IsValid` _target
    (:`Is Valid`
      (set `MovementComponent.Velocity` (* (`KismetMathLibrary.Normal` (- (`self.K2_GetActorLocation` _target) (`self.K2_GetActorLocation`))) (`ProjectileMovementComponent.InitialSpeed` _projectilemovement)) _projectilemovement))))

(event `self.Sphere.OnComponentHit`
  (params (HitComponent :type "PrimitiveComponent Object Reference") (OtherActor :type "Actor Object Reference") (OtherComp :type "PrimitiveComponent Object Reference") (NormalImpulse :type "Vector Structure") (Hit :type "HitResult Structure (by ref)"))
  ;[1 1 1] missile deals damage to enemy on collision
  (bind _asbp_dummy_eenemy (cast `/Game/BluePrints/DummyEnemy/BP_DummyEnemy` OtherActor))
  (`GameplayStatics.ApplyDamage` _asbp_dummy_eenemy 10.0)
  (`self.K2_DestroyActor`))

(fn `UserConstructionScript`)