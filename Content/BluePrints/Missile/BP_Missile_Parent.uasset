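; Parent missile Blueprint for a homing projectile that chases an assigned enemy.
; Each Tick, while the target is valid, it points the ProjectileMovement velocity straight at that enemy at initial speed.
; Overlapping any BP_DummyEnemy, not just the target, applies MissileDamage and destroys the missile.
; BeginPlay starts a timer intended to destroy the missile after several seconds, with SelfDestruct providing the destroy call.
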(event `SetTargetEnemy`
  (params (Eenemy :type "Actor Object Reference"))
  ;[1 1 1] set the target enemy
  (set `self.Target` Eenemy))

(event `self.ReceiveTick`
  (params (DeltaSeconds :type "Float (single-precision)"))
  (bind _target (`self.Target`))
  (bind _projectilemovement (`self.ProjectileMovement`))
  ;[1 1 1] add velocity so the missle can chase after the enemy
  (`/Engine/EditorBlueprintResources/StandardMacros.IsValid` _target
    (:`Is Valid`
      (set `MovementComponent.Velocity` (* (`KismetMathLibrary.Normal` (- (`self.K2_GetActorLocation` _target) (`self.K2_GetActorLocation`))) (`ProjectileMovementComponent.InitialSpeed` _projectilemovement)) _projectilemovement))))

(event `self.MIssile.OnComponentBeginOverlap`
  (params (OverlappedComponent :type "PrimitiveComponent Object Reference") (OtherActor :type "Actor Object Reference") (OtherComp :type "PrimitiveComponent Object Reference") (OtherBodyIndex :type Integer) (bFromSweep :type Boolean) (SweepResult :type "HitResult Structure (by ref)"))
  ;[1 1 1] missile deals damage to enemy on collision
  (bind _asbp_dummy_enemy (cast `/Game/BluePrints/DummyEnemy/BP_DummyEnemy` OtherActor))
  (`GameplayStatics.ApplyDamage` _asbp_dummy_enemy (`self.MissileDamage`))
  (`self.K2_DestroyActor`))

(event `self.ReceiveBeginPlay`
  ;[1 1 1] Destroy the missile after several seconds
  (`KismetSystemLibrary.K2_SetTimerDelegate` (`|CreateDelegate` :!event `SelfDestruct`) 5.0 true))

(fn `SelfDestruct`
  (`self.K2_DestroyActor`))

(fn `UserConstructionScript`)