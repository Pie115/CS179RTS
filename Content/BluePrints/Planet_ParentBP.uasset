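; Parent Blueprint for selectable planets that highlights the planet and drives the planet menu from the player controller's selection.
; Each Tick it compares itself to the controller's selected and hovered actors, setting a selected, hovered or empty overlay material.
; Two cross-resetting DoOnce nodes make menu changes fire once per transition: selection shows the summary for its PlanetName, deselection hides the planet menus.
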(event `self.ReceiveBeginPlay`
  ;[1 1 1] Initial Setup
  (bind _asbpplayer_controller (cast `/Game/Core/Player/BPPlayerController` (`GameplayStatics.GetPlayerController` 0)))
  (set `self.As BPPlayer Controller` _asbpplayer_controller))

(event `self.ReceiveTick`
  (params (DeltaSeconds :type "Float (single-precision)"))
  (bind _as_bpplayer_controller (`self.As BPPlayer Controller`))
  (bind _planet (`self.Planet`))
  (bind _wb_planetmenu (`/Game/UI/Blueprints/WB_Menus.WB_PlanetMenu` (`/Game/Core/Player/BPPlayerController.Menus` (`self.As BPPlayer Controller`))))
  (bind _wb_planetsummary (`/Game/UI/Blueprints/WB_PlanetMenu.WB_PlanetSummary` _wb_planetmenu))
  (bind _wb_planetpopulation (`/Game/UI/Blueprints/WB_PlanetMenu.WB_PlanetPopulation` _wb_planetmenu))
  ;[1 1 1] Highlight+Select+Display
  (if (== (`/Game/Core/Player/BPPlayerController.Selected Actor` _as_bpplayer_controller) self)
    (`MeshComponent.SetOverlayMaterial` _planet "/Game/TA2Project/Materials/Highlight_Selected.Highlight_Selected")
    (`|ExecutionSequence`
      (:`then_0`
        (goto _label_2 :!via `Reset`))
      (:`then_1`
        (`/Engine/EditorBlueprintResources/StandardMacros.DoOnce` false :!label _label
          (:`Completed`
            (`Widget.SetVisibility` _wb_planetmenu "Visible")
            (`Widget.SetVisibility` _wb_planetsummary "Visible")
            (`Widget.SetVisibility` _wb_planetpopulation "Hidden")
            (`/Game/UI/Blueprints/WB_PlanetMenu.ChangePlanet` _wb_planetmenu (`self.Planet Name`))))))
    (else
      (if (== (`/Game/Core/Player/BPPlayerController.Hovered Actor` _as_bpplayer_controller) self)
        (`MeshComponent.SetOverlayMaterial` _planet "/Game/TA2Project/Materials/Highlight_Hovered.Highlight_Hovered")
        (else
          (`MeshComponent.SetOverlayMaterial` _planet null)))
      (`|ExecutionSequence`
        (:`then_0`
          (goto _label :!via `Reset`))
        (:`then_1`
          (`/Engine/EditorBlueprintResources/StandardMacros.DoOnce` false :!label _label_2
            (:`Completed`
              (`Widget.SetVisibility` _wb_planetmenu "Hidden")
              (`Widget.SetVisibility` _wb_planetsummary "Hidden")
              (`Widget.SetVisibility` _wb_planetpopulation "Hidden")
              (`Widget.SetVisibility` (`/Game/UI/Blueprints/WB_PlanetSummary.WB_BuildingMenu` _wb_planetsummary) "Hidden"))))))))

(fn `UserConstructionScript`)