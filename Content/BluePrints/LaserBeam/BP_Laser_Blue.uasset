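; BP_Laser_Blue is a laser beam actor that tracks a BP_DummyEnemy and damages it continuously.
; Each tick it moves the Niagara "Beam End" parameter to the enemy and applies damage scaled by the Planet's Gunner worker count and delta time.
; Without a valid enemy, the beam end collapses to the actor's location, hiding it inside the planet.
; The SetTrackTarget event assigns the enemy but is marked unused.
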(event `SetTrackTarget`
  (params (EnemyShip :type "Actor Object Reference"))
  ;[1 1 1] UNUSED
  (bind _asbp_dummy_enemy (cast `/Game/BluePrints/DummyEnemy/BP_DummyEnemy` EnemyShip))
  (set `self.LaserEnemy` _asbp_dummy_enemy))

(event `self.ReceiveTick`
  (params (DeltaSeconds :type "Float (single-precision)"))
  (bind _laserenemy (`self.LaserEnemy`))
  ;[1 1 1] LASER TRACE THE ENEMY EVERY TICK
  (`/Engine/EditorBlueprintResources/StandardMacros.IsValid` _laserenemy
    (:`Is Valid`
      (bind _asbp_dummy_enemy (cast `/Game/BluePrints/DummyEnemy/BP_DummyEnemy` _laserenemy))
      (`self.Set Laser Target Location` (`self.K2_GetActorLocation` _asbp_dummy_enemy))
      (bind _returnvalue (`cpp_PlanetBase.GetCurrentWorker` (`self.Planet`) "Gunner"))
      (`/Game/BluePrints/DummyEnemy/BP_DummyEnemy.TakeDamage` _asbp_dummy_enemy (* 10.0 (* _returnvalue (`GameplayStatics.GetWorldDeltaSeconds`)))))
    (:`Is Not Valid`
      ;;[1 1 1] no enemy, hide the beam inside of planets
      (`self.Set Laser Target Location` (`self.K2_GetActorLocation`)))))

(fn `Set Laser Target Location`
  (params (`NewTargetLocation ` :type "Vector Structure"))
  ;[1 1 1] set beam end to a given location
  (bind _output_get (set `self.TargetLocation ` `NewTargetLocation `))
  (`FXSystemComponent.SetVectorParameter` (`self.Niagara`) "Beam End" _output_get))

(fn `UserConstructionScript`)