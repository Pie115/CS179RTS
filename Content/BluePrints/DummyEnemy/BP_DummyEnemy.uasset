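; BP_DummyEnemy is a simple enemy actor that can be damaged and deals damage on contact.
; AnyDamage routes into TakeDamage, which subtracts from Health and destroys the actor at zero or below.
; On overlap it applies BaseDamage to the other actor and then destroys itself.
; SetHealth and SetSpeed are setters, with speed stored at ten times the given value.
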(event `TakeDamage`
  (params (damageAmount :type "Float (double-precision)"))
  ;[1 1 1] calculate health after taking damage
  (set `self.health` (- (`self.health`) damageAmount))
  (if (<= (`self.health`) 0.0)
    (`self.K2_DestroyActor`)))

(event `self.ReceiveAnyDamage`
  (params (Damage :type "Float (single-precision)") (DamageType :type "DamageType Object Reference") (InstigatedBy :type "Controller Object Reference") (DamageCauser :type "Actor Object Reference"))
  (`self.TakeDamage` Damage))

(event `self.ReceiveActorBeginOverlap`
  (params (OtherActor :type "Actor Object Reference"))
  ;[1 1 1] Do collision damage
  (`GameplayStatics.ApplyDamage` OtherActor (`self.Base Damage`))
  (`self.K2_DestroyActor`))

(fn `Set Health`
  (params (NewHealth :type "Float (double-precision)"))
  (set `self.health` NewHealth))

(fn `Set Speed`
  (params (NewSpeed :type Integer))
  (set `self.Speed` (* NewSpeed 10)))

(fn `UserConstructionScript`)