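; Blue laser planet, a child planet Blueprint that attacks with a single laser beam actor.
; BeginPlay sets its range, weapon class and name before calling the parent, then spawns the beam and starts a looping timer.
; CreateWeapon spawns the beam at the planet, sets its target location to the world origin and links it back to the planet.
; SetWeaponEnemy passes the current target enemy to the beam.
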(event `self.ReceiveBeginPlay`
  ;[1 1 1] Attack Range must set before parent BeginPlay
  (set `self.AttackRange` 2000.0)
  (set `self.WeaponClass` "/Game/BluePrints/LaserBeam/BP_Laser_Blue_Parent.BP_Laser_Blue_Parent_C")
  (set `self.Planet Name` "BlueLaser")
  ;[1 1 1] Use overide function for unique weapon
  (`parent.ReceiveBeginPlay`)
  (`self.CreateWeapon`)
  (`KismetSystemLibrary.K2_SetTimerDelegate` (`|CreateDelegate` :!event `Set Weapon Enemy`) 0.4 true))

(fn `CreateWeapon`
  ;[1 1 1] Create one laser beam and set the end point in the center of the planet
  (bind _returnvalue (`|SpawnActorFromClass` (`self.WeaponClass`) (`KismetMathLibrary.MakeTransform` (`self.K2_GetActorLocation`)) "Undefined" "MultiplyWithRoot" null null))
  (bind _output_get (set `self.LaserBeam` _returnvalue))
  (bind _asbp_laser_blue_parent (cast `/Game/BluePrints/LaserBeam/BP_Laser_Blue_Parent` _output_get))
  (`/Game/BluePrints/LaserBeam/BP_Laser_Blue_Parent.Set Laser Target Location` _asbp_laser_blue_parent (0.0 0.0 0.0))
  (`KismetSystemLibrary.PrintString` "create blue laser")
  (set `/Game/BluePrints/LaserBeam/BP_Laser_Blue_Parent.Planet` self _asbp_laser_blue_parent)
  (return))

(fn `Set Weapon Enemy`
  ;[1 1 1] change the variable laser enemy inside of laserbeam
  (bind _asbp_laser_blue_parent (cast `/Game/BluePrints/LaserBeam/BP_Laser_Blue_Parent` (`self.LaserBeam`)))
  (bind _asbp_dummy_enemy (cast `/Game/BluePrints/DummyEnemy/BP_DummyEnemy` (`self.TargetEnemy`)))
  (set `/Game/BluePrints/LaserBeam/BP_Laser_Blue_Parent.LaserEnemy` _asbp_dummy_enemy _asbp_laser_blue_parent))

(fn `UserConstructionScript`
  (`parent.UserConstructionScript`))