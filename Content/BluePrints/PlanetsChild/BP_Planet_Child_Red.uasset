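; Red laser planet variant, a child of a base planet Blueprint that supplies the weapon logic.
; On BeginPlay it sets its attack range, laser weapon class and name, runs the parent BeginPlay, then creates the weapon.
; It also starts a short looping timer through an event delegate whose target is not shown here.
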(event `self.ReceiveBeginPlay`
  (set `self.AttackRange` 1000.0)
  (set `self.WeaponClass` "/Game/BluePrints/LaserBeam/BP_Laser_Red_Child.BP_Laser_Red_Child_C")
  (set `self.Planet Name` "RedLaser")
  ;[1 1 1] Ues parent weapon, the default weapon is red laser, no need to overide
  (`parent.ReceiveBeginPlay`)
  (`self.CreateWeapon`)
  (`KismetSystemLibrary.K2_SetTimerDelegate` (`|CreateDelegate` :!event `Set Weapon Enemy`) 0.4 true))

(fn `UserConstructionScript`
  (`parent.UserConstructionScript`))